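; BP_Enemy is an enemy actor that dies to projectiles and damages the player on contact.
; It removes itself after a fixed lifespan, or through a Tick check once the player's X position reaches or passes its own.
; Its overlap event destroys it on projectile hits; player hits also shake the camera and reduce health.
; When health equals exactly zero, it flags the player dead and calls DisplayRestart.
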(event OnComponentBeginOverlap(Enemy)
  (params (OverlappedComponent :type Primitive%20Component%20Object%20Reference) (OtherActor :type Actor%20Object%20Reference) (OtherComp :type Primitive%20Component%20Object%20Reference) (OtherBodyIndex :type Integer) (bFromSweep :type Boolean) (SweepResult :type Hit%20Result%20Structure%20%28by%20ref%29))
  (Utilities|FlowControl|Sequence
    (:then_0
      (Utilities|Casting|CastToBP_Projectile OtherActor)
      (Actor|DestroyActor))
    (:then_1
      (bind _asbp_player (Utilities|Casting|CastToBP_Player OtherActor))
      (Class|PlayerCameraManager|StartCameraShakefromSource (Game|GetPlayerCameraManager 0) "/Game/Blueprints/shake.shake_C" 0 1.0 "CameraLocal" "0, 0, 0")
      (Actor|DestroyActor)
      (bind _output_get (Variables|/Game/InfiniteMatrix/Blueprints/BP_Player.BP_Player_C|SetHealth _asbp_player (+ (Variables|/Game/InfiniteMatrix/Blueprints/BP_Player.BP_Player_C|GetHealth _asbp_player) -0.25)))
      (if (== _output_get 0.0)
        (Variables|/Game/InfiniteMatrix/Blueprints/BP_Player.BP_Player_C|SetIsDead _asbp_player true)
        (Default|DisplayRestart _asbp_player)))))

(event EventBeginPlay
  (Actor|SetLifeSpan 1e+01))

(event Collision|EventActorBeginOverlap
  (params (OtherActor :type Actor%20Object%20Reference)))

(event EventTick
  (params (DeltaSeconds :type Float%20%28single-precision%29))
  (bind _asbp_player (Utilities|Casting|CastToBP_Player (Game|Player|GetPlayerPawn 0)))
  (if (>= (.X (Math|Vector|BreakVector (Transformation|GetActorLocation _asbp_player))) (.X (Math|Vector|BreakVector (Transformation|GetActorLocation))))
    (Actor|DestroyActor)))

(fn ConstructionScript)