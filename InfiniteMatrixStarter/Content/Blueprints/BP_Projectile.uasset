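; BP_Projectile is a bullet actor that scores hits on enemies and removes itself on impact, with a short life span as fallback.
; The Bullet component's end-overlap event checks the other actor's type in sequence.
; An enemy adds one to the player's score and destroys the projectile.
; A tunnel destroys it only while Collision overlaps the wall mesh, and a health pack destroys it without further effect.
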(event OnComponentEndOverlap(bullet)
  (params (OverlappedComponent :type Primitive%20Component%20Object%20Reference) (OtherActor :type Actor%20Object%20Reference) (OtherComp :type Primitive%20Component%20Object%20Reference) (OtherBodyIndex :type Integer))
  (Utilities|FlowControl|Sequence
    (:then_0
      (Utilities|Casting|CastToBP_Enemy OtherActor)
      (bind _asbp_player (Utilities|Casting|CastToBP_Player (Game|Player|GetPlayerPawn 0)))
      (Variables|/Game/InfiniteMatrix/Blueprints/BP_Player.BP_Player_C|Setscore _asbp_player (+ (Variables|/Game/InfiniteMatrix/Blueprints/BP_Player.BP_Player_C|Getscore _asbp_player) 1))
      (Actor|DestroyActor))
    (:then_1
      (bind _asbp_tunnel (Utilities|Casting|CastToBP_Tunnel OtherActor))
      (if (Class|PrimitiveComponent|IsOverlappingComponent (Variables|Default|Getcollision) (Variables|/Game/InfiniteMatrix/Blueprints/BP_Tunnel.BP_Tunnel_C|GetWallMesh _asbp_tunnel))
        (Actor|DestroyActor)))
    (:then_2
      (Utilities|Casting|CastToBP_HealthPack OtherActor)
      (Actor|DestroyActor))))

(event EventBeginPlay
  (Actor|SetLifeSpan 2.0))

(event Collision|EventActorBeginOverlap
  (params (OtherActor :type Actor%20Object%20Reference)))

(event EventTick
  (params (DeltaSeconds :type Float%20%28single-precision%29)))

(fn ConstructionScript)

(fn Destroy
  (Actor|DestroyActor))